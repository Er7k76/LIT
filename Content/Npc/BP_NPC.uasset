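; Interactable dialogue NPC that turns to face the player and starts conversations through the Bp_WordManager game instance.
; Interact registers it as the current NPC, captures the look-at yaw, blends the camera view to it and starts its dialogue, or an alternate one if a required word is unlearned.
; Tick interpolates the skeletal mesh toward that yaw, or back to the actor's initial rotation once NPCRotate clears the facing flag.
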(event `self.ReceiveTick`
  (params (DeltaSeconds :type "Float (single-precision)"))
  (bind (`_rotaçao_inicial_roll` `_rotaçao_inicial_pitch` `_rotaçao_inicial_yaw`) (`KismetMathLibrary.BreakRotator` (`self.Rotaçao_Inicial`)))
  (bind (_target_location_roll _target_location_pitch _target_location_yaw) (`KismetMathLibrary.BreakRotator` (`self.Target_location`)))
  (bind _returnvalue (`SceneComponent.K2_GetComponentRotation` (`self.SkeletalMesh`)))
  (bind _returnvalue_2 (`SceneComponent.K2_GetComponentRotation` (`self.SkeletalMesh`)))
  (bind _returnvalue_3 (`KismetMathLibrary.RInterpTo` _returnvalue_2 (`KismetMathLibrary.MakeRotator` 0.0 0.0 _target_location_yaw) DeltaSeconds 5.0))
  (bind _returnvalue_4 (`KismetMathLibrary.RInterpTo` _returnvalue (`KismetMathLibrary.MakeRotator` `_rotaçao_inicial_roll` `_rotaçao_inicial_pitch` `_rotaçao_inicial_yaw`) DeltaSeconds 5.0))
  (if (`self.b_player_Rotate`)
    (`SceneComponent.K2_SetWorldRotation` (`self.SkeletalMesh`) _returnvalue_3 false false)
    (if (== _returnvalue_3 _returnvalue_2 :`ErrorTolerance` 0.2)
      _)
    (elif true
      (`SceneComponent.K2_SetWorldRotation` (`self.SkeletalMesh`) _returnvalue_4 false false)
      (if (== _returnvalue_4 _returnvalue :`ErrorTolerance` 0.2)
        (set `self.b_base_rotate` false)))))

(event `self.ReceiveBeginPlay`
  (set `self.Rotaçao_Inicial` (`self.K2_GetActorRotation`)))

(event `/Game/Npc/BPI_Interactable.Interact`
  (bind (_returnvalue_x _returnvalue_y _returnvalue_z) (`KismetMathLibrary.BreakVector` (`self.K2_GetActorLocation` (`Controller.K2_GetPawn` (`GameplayStatics.GetPlayerController` 0)))))
  (bind _asbp_word_manager (cast `/Game/Dialogue_system/Bp_WordManager` (`GameplayStatics.GetGameInstance`)))
  (set `/Game/Dialogue_system/Bp_WordManager.Curent_Npc` self _asbp_word_manager)
  (set `self.Target_location` (`KismetMathLibrary.FindLookAtRotation` (`SceneComponent.K2_GetComponentLocation` (`self.SkeletalMesh`)) (`KismetMathLibrary.MakeVector` _returnvalue_x _returnvalue_y _returnvalue_z)))
  (set `self.b_player_Rotate` true)
  (`PlayerController.SetViewTargetWithBlend` (`GameplayStatics.GetPlayerController` 0) self 2.0 "VTBlend_PreBlended" 0.0 true)
  (bind _asbp_word_manager_2 (cast `/Game/Dialogue_system/Bp_WordManager` (`GameplayStatics.GetGameInstance`)))
  (if (`self.BRequiresWord`)
    (bind _learned (`/Game/Dialogue_system/Bp_WordManager.IsWordLearned` _asbp_word_manager_2 (`self.RequiredWord`)))
    (if _learned
      (`/Game/Dialogue_system/Bp_WordManager.StartDialogue` _asbp_word_manager_2 (`self.DialogueID`) :!label _label)
      (else
        (`/Game/Dialogue_system/Bp_WordManager.StartDialogue` _asbp_word_manager_2 (`self.WrongID`))))
    (else
      (goto _label))))

(event `/Game/Npc/BPI_Interactable.NPC_Rotate`
  (set `self.b_player_Rotate` false)
  (set `self.b_base_rotate` true))

(event `self.SkeletalMesh.OnAnimInitialized`
  (`KismetSystemLibrary.PrintString` "Começou animaçao"))

(fn `UserConstructionScript`)