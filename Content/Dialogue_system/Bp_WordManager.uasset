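; Word manager Blueprint that tracks the player's language learning and also handles dialogue and a simple inventory.
; Symbol and meaning discovery copy word-table rows into a progress array, set learned flags and register IDs as learned words.
; Dialogue rows are looked up by ID and can open a dialogue widget.
; Inventory stores only item IDs; added quantities are not saved and HasItem ignores required quantity.
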(fn `AddItem`
  (params (ItemID :type Name) (Quantitytoadd :type Integer))
  (bind _returnvalue (`|GetDataTableRow` (`self.ItensDataTable`) ItemID)
    (:`then`
      (set `self.bitemfound` false)
      (for _array_element (`self.InventoryItens`)
        (bind (_item_id _item_name _item_icon _item_quantity) (break `/Game/Inventory_System/ST_Itens` _returnvalue))
        (if (== _array_element _item_id)
          (set `self.bitemfound` true)
          (setmembers `/Game/Inventory_System/ST_Itens` :`StructRef` _returnvalue :`Item_ID` "None" :`Item_name` "" :`Item_Icon` null :`Item_quantity` (+ _item_quantity Quantitytoadd) :`bstackble` false)
          (else
            (`KismetArrayLibrary.Array_AddUnique` (`self.InventoryItens`) ItemID)
            (for _ (`self.InventoryItens`)
              _)))))))

(fn `DiscoverSymbool`
  (params (WordID :type Name))
  (bind _wordpogress (`self.WordPogress`))
  (bind _returnvalue (`|GetDataTableRow` (`self.WordDataTable`) WordID)
    (:`then`
      (for (_array_element _array_index) (`self.WordPogress`)
        (if (== WordID (`.WordID_2_97B0707346C293312FE658AFAC3BA724` (break `/Game/Dialogue_system/St_word` _array_element)))
          (bind _structout (setmembers `/Game/Dialogue_system/St_word` :`StructRef` _array_element :`Simbolo_Learned` true))
          (`KismetArrayLibrary.Array_Set` (`self.WordPogress`) _array_index _structout)
          (`self.LearnWord` WordID :!label _label)))
      (bind _structout_2 (setmembers `/Game/Dialogue_system/St_word` :`StructRef` _returnvalue :`Simbolo_Learned` true))
      (`KismetArrayLibrary.Array_AddUnique` _wordpogress _structout_2)
      (`KismetArrayLibrary.Array_Set` _wordpogress _array_index _structout_2)
      (goto _label))))

(fn `GetDialogue`
  (params (DialogueID :type Name))
  (returns (RowFound :type Boolean) (Dialogue :type "/Game/Dialogue_system/ST_Dialogueline Structure"))
  (bind _returnvalue (`|GetDataTableRow` (`self.DialogueDataTable`) DialogueID)
    (:`then`
      (return true _returnvalue))
    (:`RowNotFound`
      (return false))))

(fn `GetLearnedWords`
  (returns (LearnedWords :type "Array of Name"))
  (return (`self.LearneedWords`)))

(fn `GetWord`
  (params (Wordid :type Name))
  (returns (Word :type "/Game/Dialogue_system/St_word Structure"))
  (for _array_element (`self.WordPogress`)
    (if (== Wordid (`.WordID_2_97B0707346C293312FE658AFAC3BA724` (break `/Game/Dialogue_system/St_word` _array_element)))
      (return _array_element))))

(fn `HasItem`
  (params (ItemID :type Name) (RequiresQuantity :type Integer))
  (returns (HasItem :type Boolean))
  (for _array_element (`self.InventoryItens`)
    (bind _returnvalue (`|GetDataTableRow` (`self.ItensDataTable`) _array_element)
      (:`then`
        (if (== (`.Item_ID_2_64357A344813A4585B417BA70935BEFE` (break `/Game/Inventory_System/ST_Itens` _returnvalue)) ItemID)
          (return true)
          (else
            (return false)))))))

(fn `IsWordLearned`
  (params (Wordid :type Name))
  (returns (Learned :type Boolean))
  (if (`KismetArrayLibrary.Array_Contains` (`self.LearneedWords`) Wordid)
    (return true)
    (else
      (return false))))

(fn `LearnMeanoing`
  (params (WordId :type Name))
  (bind _wordpogress (`self.WordPogress`))
  (bind _returnvalue (`|GetDataTableRow` (`self.WordDataTable`) WordId)
    (:`then`
      (for (_array_element _array_index) (`self.WordPogress`)
        (if (== WordId (`.WordID_2_97B0707346C293312FE658AFAC3BA724` (break `/Game/Dialogue_system/St_word` _array_element)))
          (bind _structout (setmembers `/Game/Dialogue_system/St_word` :`StructRef` _array_element :`Simbolo_Learned` true :`Meaning_Learned` true))
          (`KismetArrayLibrary.Array_Set` (`self.WordPogress`) _array_index _structout)
          (`self.LearnWord` WordId :!label _label)))
      (bind _structout_2 (setmembers `/Game/Dialogue_system/St_word` :`StructRef` _returnvalue :`Simbolo_Learned` true :`Meaning_Learned` true))
      (`KismetArrayLibrary.Array_AddUnique` _wordpogress _structout_2)
      (`KismetArrayLibrary.Array_Set` _wordpogress _array_index _structout_2)
      (goto _label))))

(fn `LearnWord`
  (params (Wordid :type Name))
  (bind _learneedwords (`self.LearneedWords`))
  (if (`KismetArrayLibrary.Array_Contains` (`self.LearneedWords`) Wordid)
    (return)
    (else
      (`KismetArrayLibrary.Array_AddUnique` _learneedwords Wordid)
      (for _array_element _learneedwords
        (`KismetSystemLibrary.PrintString` (`KismetStringLibrary.Conv_NameToString` _array_element))))))

(fn `StartDialogue`
  (params (DialogueID :type Name))
  (bind _returnvalue (`|GetDataTableRow` (`self.DialogueDataTable`) DialogueID)
    (:`then`
      (bind _returnvalue_2 (`|CreateWidget` "/Game/Dialogue_system/WBP_Dialogue.WBP_Dialogue_C" null _returnvalue))
      (`UserWidget.AddToViewport` _returnvalue_2 0))))